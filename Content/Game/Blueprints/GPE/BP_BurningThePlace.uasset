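; Interactable that burns the place down, swapping the casino and lab streamed levels for the fire-ending level behind a fade.
; Fire sound plays during the interaction and stops on cancel; completion flags the player as inspecting, destroys a target actor and attaches movable actors to BP_BoatRoot.
; After the fade, it releases the player and sets the volume of the first "Fire"-tagged actor's audio, cached at BeginPlay.
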(event OnInteractionBegin(Manager_InteractionTarget)
  (params (InteractorPawn :type Pawn%20Object%20Reference))
  (Audio|Components|Audio|Play (Variables|Default|GetFireSound) 0.0))

(event OnInteractionEnd(Manager_InteractionTarget)
  (params (Result :type Enum_InteractionResult%20Enum :default "NewEnumerator0") (InteractorPawn :type Pawn%20Object%20Reference))
  (bind _wbp_fade (Variables|Default|GetWBP_Fade))
  (bind _asbp_player (Utilities|Casting|CastToBP_Player InteractorPawn))
  (Variables|Default|SetAs%20BP%20Player _asbp_player)
  (switch Utilities|FlowControl|Switch|SwitchonEnum_InteractionResult Result
    (:NewEnumerator0
      (UserInterface|Viewport|AddtoViewport _wbp_fade 0)
      (Default|PlayFade _wbp_fade)
      (Utilities|FlowControl|Delay 1.0)
      (Utilities|FlowControl|Sequence
        (:then_0
          (Variables|/Game/Game/Blueprints/BP_Player.BP_Player_C|SetisInspectingItem (Variables|Default|GetAs%20BP%20Player) true)
          (Class|GameplayStatics|LoadStreamLevelbySoftObjectPtr "/Game/Game/Levels/L_FireEnd.L_FireEnd" true false)
          (Class|GameplayStatics|UnloadStreamLevelbySoftObjectPtr "/Game/Game/Levels/L_Casino.L_Casino" false)
          (Class|GameplayStatics|UnloadStreamLevelbySoftObjectPtr "/Game/Game/Levels/Labo_Build.Labo_Build" false)
          (bind _returnvalue (Actor|GetActorOfClass "/Game/Game/Blueprints/BP_BoatRoot.BP_BoatRoot_C"))
          (bind _outactors (Actor|GetAllActorsOfClass "/Script/Engine.Actor"))
          (for _array_element _outactors
            (Utilities|IsValid (Variables|/Script/Engine.Actor|GetRootComponent _array_element)
              (:Is%20Valid
                (if (and (Utilities|Enum|Equal(Enum) (Utilities|String|EnumtoString (Variables|/Script/Engine.SceneComponent|GetMobility (Variables|/Script/Engine.Actor|GetRootComponent _array_element))) "Movable") (!= _array_element _returnvalue))
                  (Transformation|AttachActorToActor _array_element _returnvalue "None" "KeepRelative" "KeepRelative" "KeepWorld" true))))))
        (:then_1
          (Actor|DestroyActor (Variables|Default|GetActorToDestroy))
          (Utilities|FlowControl|Delay (Variables|Default|GetFadeDuration))
          (Audio|Components|Audio|FadeOut (Variables|Default|GetFireSound) 5.0 0.0 "Linear" :!class /Script/Engine.AudioComponent)
          (Default|RemoveFade _wbp_fade)
          (Utilities|FlowControl|Delay 1.0)
          (Widget|RemovefromParent _wbp_fade)
          (Variables|/Game/Game/Blueprints/BP_Player.BP_Player_C|SetisInspectingItem (Variables|Default|GetAs%20BP%20Player) false)
          (Audio|Components|Audio|SetVolumeMultiplier (Actor|GetComponentbyClass (Utilities|Array|Get(acopy) (Variables|Default|GetAudioFire)) "/Script/Engine.AudioComponent") 1.0 :!class /Script/Engine.AudioComponent))))
    (:NewEnumerator1
      (Audio|Components|Audio|Stop (Variables|Default|GetFireSound)))))

(event EventBeginPlay
  (Class|GameplayStatics|UnloadStreamLevelbySoftObjectPtr "/Game/Game/Levels/L_Fire.L_Fire" false)
  (bind _outactors (Actor|GetAllActorswithTag "Fire"))
  (Variables|Default|SetAudioFire _outactors))

(event Collision|EventActorBeginOverlap
  (params (OtherActor :type Actor%20Object%20Reference)))

(event EventTick
  (params (DeltaSeconds :type Float%20%28single-precision%29)))

(fn ConstructionScript)