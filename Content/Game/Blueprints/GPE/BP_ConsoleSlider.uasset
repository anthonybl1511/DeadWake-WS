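; BP_ConsoleSlider is a puzzle console that checks whether a set of sliders matches a target combination.
; BeginPlay fills an Indicators array from three indicator components.
; CheckPos compares each slider's PointIndex to the Combination entry at that index, turning its indicator emissive green or red.
; It counts matches, only prints "Done" when all three are correct, then resets the score.
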(event Custom|CheckPos
  (bind (_array_element _array_index) (Utilities|Array|ForEachLoopwithBreak (Variables|Default|GetSliders))
    (:LoopBody
      (if (== (Variables|/Game/Game/Blueprints/GPE/BP_Slider.BP_Slider_C|GetPoint%20Index _array_element) (Utilities|Array|Get(acopy) (Variables|Default|GetCombination) _array_index))
        (Rendering|Material|SetMaterial (Utilities|Array|Get(acopy) (Variables|Default|GetIndicators) _array_index) 0 "/Game/Game/Assets/Materials/MI_GreenEmissive.MI_GreenEmissive")
        (bind _result (Math|Integer|IncrementInt (Variables|Default|GetCorrectScore))
          (:%20%20
            (if (== _result 3)
              (Development|PrintString "Done"))))
        (else
          (Rendering|Material|SetMaterial (Utilities|Array|Get(acopy) (Variables|Default|GetIndicators) _array_index) 0 "/Game/Game/Assets/Materials/MI_RedEmissive.MI_RedEmissive"))))
    (:Completed
      (Variables|Default|SetCorrectScore 0))))

(event Collision|EventActorBeginOverlap
  (params (OtherActor :type Actor%20Object%20Reference)))

(event EventTick
  (params (DeltaSeconds :type Float%20%28single-precision%29)))

(event EventBeginPlay
  (bind _indicators (Variables|Default|GetIndicators))
  (Utilities|Array|SetArrayElem _indicators 0 (Variables|Default|GetIndicator1) true)
  (Utilities|Array|SetArrayElem _indicators 1 (Variables|Default|GetIndicator2) true)
  (Utilities|Array|SetArrayElem _indicators 2 (Variables|Default|GetIndicator3) true)
  (Development|PrintString (Utilities|GetDisplayName (Utilities|Array|Get(acopy) _indicators))))

(fn ConstructionScript)