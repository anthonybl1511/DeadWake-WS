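; BP_EndGame is an end-game actor that streams in the L_Fire level when its interaction begins.
; BeginPlay unloads L_Fire, and the interaction target's OnInteractionBegin starts a non-blocking load of it as visible.
; After a FadeDuration delay it removes the fade widget, though the nodes that would show and play that fade are disconnected.
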(event OnInteractionBegin(Manager_InteractionTarget)
  (params (InteractorPawn :type Pawn%20Object%20Reference))
  (bind _wbp_fade (Variables|Default|GetWBP_Fade))
  (Class|GameplayStatics|LoadStreamLevelbySoftObjectPtr "/Game/Game/Levels/L_Fire.L_Fire" true false)
  (Development|PrintString "level loaded")
  (Utilities|FlowControl|Delay (Variables|Default|GetFadeDuration))
  (Default|RemoveFade _wbp_fade)
  (Widget|RemovefromParent _wbp_fade))

(event EventBeginPlay
  (Class|GameplayStatics|UnloadStreamLevelbySoftObjectPtr "/Game/Game/Levels/L_Fire.L_Fire" false))

(event Collision|EventActorBeginOverlap
  (params (OtherActor :type Actor%20Object%20Reference)))

(event EventTick
  (params (DeltaSeconds :type Float%20%28single-precision%29)))

(fn ConstructionScript)