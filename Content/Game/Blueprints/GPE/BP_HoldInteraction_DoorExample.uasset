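; Example hold-interaction door: players insert a carried wheel into a slot, then hold the valve to open it.
; Insertion consumes the item, animates the wheel in and moves collision targets to expose the valve interaction.
; Hold progress scales the door and spins the wheel, multicast with sound, skipping re-application on the locally controlled interactor.
; Completion multicasts disabling the blocking volume's collision, while cancellation plays the door timeline in reverse.
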(event OnInteractionEnd(Manager_InteractionTarget)
  (params (Result :type Enum_InteractionResult%20Enum :default "NewEnumerator0") (InteractorPawn :type Pawn%20Object%20Reference))
  (bind _wheel (Variables|Default|GetWheel))
  (bind _asbp_player (Utilities|Casting|CastToBP_Player InteractorPawn))
  (if (Utilities|String|Contains (Variables|/Game/Game/Blueprints/BP_Player.BP_Player_C|GetpickedItem _asbp_player) "Wheel")
    (Default|RemoveItem _asbp_player)
    (Utilities|FlowControl|DoOnce false
      (:Completed
        (Utilities|FlowControl|Sequence
          (:then_0
            (Rendering|SetVisibility _wheel true false)
            (Development|SetHiddeninGame _wheel false false)
            (Transformation|SetRelativeLocation (Variables|Default|GetCollisionTarget) "0.000000,0.000000,1000.000000" true false)
            (Audio|PlaySoundatLocation "/Game/Game/SFX/SFX_ValveInsertion_Cue.SFX_ValveInsertion_Cue" (Transformation|GetWorldLocation (Variables|Default|GetWheelSlot)) "0, 0, 0" 1.0 1.0 0.0 0 0 0 0)
            (bind _newtrack_0 (Timeline|Timeline PlayFromStart)
              (:Update
                (Transformation|SetRelativeLocation (Variables|Default|GetCollisionTargetValve) (Math|Vector|Lerp(Vector) "500.000000,120.000000,1697.000002" "500.000000,120.000000,-3.000000" _newtrack_0) false false))))
          (:then_1
            (bind _alpha (Timeline|ValveAnimInsert PlayFromStart)
              (:Update
                (Transformation|SetRelativeLocation _wheel (Math|Vector|Lerp(Vector) "517.000000,74.000000,57.000000" "517.000000,44.000000,57.000000" _alpha) false false)))))))
    (else
      (Audio|PlaySoundatLocation "/Game/Game/SFX/SFX_NoValve_Cue.SFX_NoValve_Cue" (Transformation|GetWorldLocation (Variables|Default|GetWheelSlot)) "0, 0, 0" 1.0 1.0 0.0 0 0 0 0))))

(event OnInteractionUpdated(Manager_InteractionTarget_Valve)
  (params (Alpha :type Float%20%28double-precision%29) (Repeated :type Integer) (InteractorPawn :type Pawn%20Object%20Reference))
  (Networking|SwitchHasAuthority
    (:Authority
      (CallFunction|UpdateCosmeticTransform Alpha)
      (CallFunction|MulticastUpdateCosmeticTransform InteractorPawn Alpha))
    (:Remote
      (CallFunction|UpdateCosmeticTransform Alpha))))

(event OnInteractionEnd(Manager_InteractionTarget_Valve)
  (params (Result :type Enum_InteractionResult%20Enum :default "NewEnumerator0") (InteractorPawn :type Pawn%20Object%20Reference))
  (bind _gatesound (Variables|Default|GetGateSound))
  (Utilities|FlowControl|Sequence
    (:then_0
      (Audio|Components|Audio|Stop _gatesound)
      (switch Utilities|FlowControl|Switch|SwitchonEnum_InteractionResult Result
        (:NewEnumerator0
          (CallFunction|MulticastSetCollisionEnabled (Variables|Default|GetBlockingVolume)))
        (:NewEnumerator1
          (Components|Timeline|ReversefromEnd (Variables|Default|GetDoor_Timeline)))))
    (:then_1
      (Utilities|FlowControl|DoOnce false) ; enters at Reset
    )))

(event Custom|Multicast_Update_Cosmetic_Transform
  (params (Target :type Pawn%20Object%20Reference) (Alpha :type Float%20%28single-precision%29))
  (Utilities|FlowControl|Sequence
    (:then_0
      (if (not (Pawn|IsLocallyControlled Target))
        (CallFunction|UpdateCosmeticTransform Alpha)))
    (:then_1
      (Utilities|FlowControl|DoOnce false
        (:Completed
          (Audio|Components|Audio|Play (Variables|Default|GetGateSound) 0.0))))))

(event Custom|Update_Cosmetic_Transform
  (params (Alpha :type Float%20%28single-precision%29))
  (bind _output_get (Variables|Default|SetLastDoorScale (Math|Vector|Lerp(Vector) "1.100000,1.000000,1.030000" "0.200000,1.000000,1.030000" Alpha)))
  (Transformation|SetRelativeScale3D (Variables|Default|GetDoor) _output_get)
  (bind _output_get_2 (Variables|Default|SetLastWheelRotation (Math|Rotator|Lerp(Rotator) "0, 0, 0" "-360.000000,0.000000,0.000000" Alpha)))
  (Transformation|SetRelativeRotation (Variables|Default|GetWheel) _output_get_2 false false))

(event Custom|Multicast_Set_Collision_Enabled
  (params (CollisionTarget :type Primitive%20Component%20Object%20Reference))
  (Collision|SetCollisionEnabled CollisionTarget "NoCollision"))

(fn ConstructionScript)