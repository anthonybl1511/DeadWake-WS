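; BP_Incubator is an interactable that deactivates incubators and reports it to the end-game actor.
; On BeginPlay it caches actors tagged "Incubator" and the BP_EndGame instances.
; On interaction it restarts the DeactivatingAnim timeline inside a loop over those incubators, lerping the Multiplier material parameter on the loop element's first static mesh to zero.
; When the timeline finishes, it sets the Incubator flag on the first BP_EndGame.
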(event OnInteractionBegin(Manager_InteractionTarget)
  (params (InteractorPawn :type Pawn%20Object%20Reference))
  (for _array_element (Variables|Default|GetIncubators)
    (bind _alpha (Timeline|DeactivatingAnim PlayFromStart)
      (:Update
        (Rendering|Material|SetScalarParameterValueonMaterials (Utilities|Array|Get(acopy) (Actor|GetComponentsByClass _array_element "/Script/Engine.StaticMeshComponent")) "Multiplier" (Math|Float|Lerp (Variables|Default|GetInitialEmissiveValue) 0.0 _alpha)))
      (:Finished
        (Variables|/Game/Game/Blueprints/GPE/BP_EndGame.BP_EndGame_C|SetIncubator (Utilities|Array|Get(acopy) (Variables|Default|GetEndGame)) true)))))

(event EventBeginPlay
  (bind _outactors (Actor|GetAllActorswithTag "Incubator"))
  (Variables|Default|SetIncubators _outactors)
  (bind _outactors_2 (Actor|GetAllActorsOfClass "/Game/Game/Blueprints/GPE/BP_EndGame.BP_EndGame_C"))
  (Variables|Default|SetEndGame _outactors_2))

(event Collision|EventActorBeginOverlap
  (params (OtherActor :type Actor%20Object%20Reference)))

(event EventTick
  (params (DeltaSeconds :type Float%20%28single-precision%29)))

(fn ConstructionScript)