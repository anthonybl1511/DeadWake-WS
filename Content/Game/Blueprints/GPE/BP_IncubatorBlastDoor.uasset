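; Incubator blast door that swings open on its pivot, triggered either by player interaction or by a four-slot combination puzzle.
; GetSlotState records each slot's state and calls OpenDoor when four entries match the slot machine combination.
; OpenDoor plays a gate sound and runs a timeline that lerps the pivot from its current rotation toward a yaw offset computed at BeginPlay.
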(event OnInteractionBegin(Manager_InteractionTarget)
  (params (InteractorPawn :type Pawn%20Object%20Reference))
  (CallFunction|OpenDoor))

(event Custom|OpenDoor
  (bind _pivot (Variables|Default|GetPivot))
  ;[1 0.05451 0] heavy metal door opening sound
  (Audio|PlaySoundatLocation "/Game/Game/SFX/SFX_OpenSecurityGate.SFX_OpenSecurityGate" (Transformation|GetActorLocation) "0, 0, 0" 1.0 1.0 0.0 0 0 0 0)
  (bind _alpha (Timeline|DoorAnim PlayFromStart)
    (:Update
      (Transformation|SetRelativeRotation _pivot (Math|Rotator|Lerp(Rotator) (Variables|/Script/Engine.SceneComponent|GetRelativeRotation _pivot) (Variables|Default|GetFinalRot) _alpha true) false false))))

(event EventBeginPlay
  (bind _pivot (Variables|Default|GetPivot))
  (bind _relativerotation (Variables|/Script/Engine.SceneComponent|GetRelativeRotation _pivot))
  (bind (_roll _pitch _yaw) (Math|Rotator|BreakRotator _relativerotation))
  (Variables|Default|SetFinalRot (Math|Rotator|MakeRotator _roll _pitch (- _yaw 85.0))))

(event Collision|EventActorBeginOverlap
  (params (OtherActor :type Actor%20Object%20Reference)))

(event EventTick
  (params (DeltaSeconds :type Float%20%28single-precision%29)))

(fn ConstructionScript)

(fn GetSlotState
  (params (ID :type Integer) (State :type Boolean))
  (Utilities|Array|SetArrayElem (Variables|Default|GetCurrentCombination) ID State)
  (Variables|Default|SetCorrectSlot 0)
  (for (_array_element _array_index) (Variables|Default|GetSlotMachineCombination)
    (if (== _array_element (Utilities|Array|Get(acopy) (Variables|Default|GetCurrentCombination) _array_index))
      (bind _result (Math|Integer|IncrementInt (Variables|Default|GetCorrectSlot))
        (:%20%20
          (if (== _result 4)
            (CallFunction|OpenDoor)))))))