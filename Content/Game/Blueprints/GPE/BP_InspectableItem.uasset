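; BP_InspectableItem is a placeable interactable prop that the player can inspect, optionally as a pickup.
; The construction script applies the ItemModel mesh to its static mesh component.
; When the interaction target component reports the end of an interaction, it casts the pawn to BP_Player and calls InspectItem with the model, itself and the IsPickUp flag.
; An EnableInteractionAgain event turns interaction back on.
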(event OnInteractionEnd(Manager_InteractionTarget)
  (params (Result :type Enum_InteractionResult%20Enum :default "NewEnumerator0") (InteractorPawn :type Pawn%20Object%20Reference))
  (bind _asbp_player (Utilities|Casting|CastToBP_Player InteractorPawn))
  (Default|InspectItem _asbp_player (Variables|Default|GetitemModel) self (Variables|Default|GetisPickUp)))

(event Custom|EnableInteractionAgain
  (Default|EnableInteraction (Variables|Default|GetManager_InteractionTarget) true))

(fn ConstructionScript
  (Components|StaticMesh|SetStaticMesh (Variables|Default|GetStaticMesh) (Variables|Default|GetitemModel)))