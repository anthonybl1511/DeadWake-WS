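; BP_LabDoor is the laboratory door, which opens once the slot machine combination is solved.
; GetSlotState records each slot's state and calls OpenDoor when four entries match the target combination.
; OpenDoor plays a cue, async-streams in Labo_Build and attaches movable actors to BP_BoatRoot.
; Within that actor loop it also plays door audio and starts a Timeline that lerps Pivot toward a yaw offset computed at BeginPlay.
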(event Custom|OpenDoor
  (bind _pivot (Variables|Default|GetPivot))
  (Audio|PlaySound2D "/Game/Game/SFX/SFX_LabOpenCue.SFX_LabOpenCue" 1.0 1.0 0.0 0 0)
  (Class|GameplayStatics|LoadStreamLevelbySoftObjectPtr "/Game/Game/Levels/Labo_Build.Labo_Build" true false)
  (bind _returnvalue (Actor|GetActorOfClass "/Game/Game/Blueprints/BP_BoatRoot.BP_BoatRoot_C"))
  (bind _outactors (Actor|GetAllActorsOfClass "/Script/Engine.Actor"))
  (for _array_element _outactors
    (Utilities|IsValid (Variables|/Script/Engine.Actor|GetRootComponent _array_element)
      (:Is%20Valid
        (if (and (Utilities|Enum|Equal(Enum) (Utilities|String|EnumtoString (Variables|/Script/Engine.SceneComponent|GetMobility (Variables|/Script/Engine.Actor|GetRootComponent _array_element))) "Movable") (!= _array_element _returnvalue))
          (Transformation|AttachActorToActor _array_element _returnvalue "None" "KeepRelative" "KeepRelative" "KeepWorld" true)
          ;[1 0 0.03409] heavy metal door opening sound
          (Audio|Components|Audio|Play (Variables|Default|GetAudio) 0.0)
          (for _array_element_2 (Variables|Default|GetSlotMachines)
            _)
          (bind _alpha (Timeline|Timeline PlayFromStart)
            (:Update
              (Transformation|SetRelativeRotation _pivot (Math|Rotator|Lerp(Rotator) (Variables|/Script/Engine.SceneComponent|GetRelativeRotation _pivot) (Variables|Default|GetFinalRot) _alpha true) false false))))))))

(event Collision|EventActorBeginOverlap
  (params (OtherActor :type Actor%20Object%20Reference)))

(event EventTick
  (params (DeltaSeconds :type Float%20%28single-precision%29)))

(event EventBeginPlay
  (bind _pivot (Variables|Default|GetPivot))
  (bind _relativerotation (Variables|/Script/Engine.SceneComponent|GetRelativeRotation _pivot))
  (bind (_roll _pitch _yaw) (Math|Rotator|BreakRotator _relativerotation))
  (Variables|Default|SetFinalRot (Math|Rotator|MakeRotator _roll _pitch (- _yaw (Variables|Default|GetDoorRotation))))
  (bind _outactors (Actor|GetAllActorsOfClass "/Game/Game/Blueprints/GPE/BP_SlotMachine.BP_SlotMachine_C"))
  (Variables|Default|SetSlotMachines _outactors))

(fn ConstructionScript)

(fn GetSlotState
  (params (ID :type Integer) (State :type Boolean))
  (Utilities|Array|SetArrayElem (Variables|Default|GetCurrentCombination) ID State)
  (Variables|Default|SetCorrectSlot 0)
  (for (_array_element _array_index) (Variables|Default|GetSlotMachineCombination)
    (if (== _array_element (Utilities|Array|Get(acopy) (Variables|Default|GetCurrentCombination) _array_index))
      (bind _result (Math|Integer|IncrementInt (Variables|Default|GetCorrectSlot))
        (:%20%20
          (if (== _result 4)
            (CallFunction|OpenDoor)))))))