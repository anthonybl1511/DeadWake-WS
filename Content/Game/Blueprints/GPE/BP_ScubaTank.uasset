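; BP_ScubaTank is an interactable scuba tank that ends the game when the player finishes using it.
; Its interaction target component starts a WearingSuit sound or effect when interaction begins and stops it if canceled.
; On completion it shows a fade widget, plays an endgame sound, waits a configurable delay, then opens the main menu level.
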(event OnInteractionEnd(Manager_InteractionTarget)
  (params (Result :type Enum_InteractionResult%20Enum :default "NewEnumerator0") (InteractorPawn :type Pawn%20Object%20Reference))
  (bind _wbp_fade (Variables|Default|GetWBP_Fade))
  (switch Utilities|FlowControl|Switch|SwitchonEnum_InteractionResult Result
    (:NewEnumerator0
      (UserInterface|Viewport|AddtoViewport _wbp_fade 0)
      (Default|PlayFade _wbp_fade)
      (Audio|PlaySound2D "/Game/Game/SFX/Sfx_Forgotten_endgameShortv3.Sfx_Forgotten_endgameShortv3" 1.0 1.0 0.0 0 0)
      (Utilities|FlowControl|Delay (Variables|Default|GetDelayBeforeBackMenu))
      ;[1 0 0.05574] END OF GAME
      (Game|OpenLevel(byObjectReference) "/Game/Game/Levels/L_MainMenu.L_MainMenu"))
    (:NewEnumerator1
      (Audio|Components|Audio|Stop (Variables|Default|GetWearingSuit)))))

(event OnInteractionBegin(Manager_InteractionTarget)
  (params (InteractorPawn :type Pawn%20Object%20Reference))
  (Audio|Components|Audio|Play (Variables|Default|GetWearingSuit) 0.0))

(event EventBeginPlay)

(event Collision|EventActorBeginOverlap
  (params (OtherActor :type Actor%20Object%20Reference)))

(event EventTick
  (params (DeltaSeconds :type Float%20%28single-precision%29)))

(fn ConstructionScript)