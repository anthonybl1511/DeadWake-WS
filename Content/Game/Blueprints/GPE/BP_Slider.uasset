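; BP_Slider is an interactable puzzle slider that steps through points on a spline, linked to a BP_ConsoleSlider found in the level at BeginPlay.
; While the console is not activated, each interaction plays a switch sound, advances the point index and has the console check positions, then wraps the index after the fifth point.
; A sped-up timeline lerps the slider to the indexed spline point, and CheckPos exposes the current index.
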(event OnInteractionBegin(Manager_InteractionTarget)
  (params (InteractorPawn :type Pawn%20Object%20Reference))
  (if (not (Variables|/Game/Game/Blueprints/GPE/BP_ConsoleSlider.BP_ConsoleSlider_C|GetActivated (Variables|Default|GetConsole)))
    (Audio|PlaySoundatLocation "/Game/Game/SFX/SFX_Switch1.SFX_Switch1" (Transformation|GetActorLocation) "0, 0, 0" 1.0 1.0 0.2 0 0 0 0)
    (Math|Integer|IncrementInt (Variables|Default|GetPoint%20Index)
      (:%20%20
        (Default|CheckPos (Variables|Default|GetConsole))
        (if (>= (Variables|Default|GetPoint%20Index) 5)
          (Variables|Default|SetPoint%20Index 0)
          (bind _alpha (Timeline|SliderAnim PlayFromStart)
            (:Update
              (Transformation|SetRelativeLocation (Variables|Default|GetSlider) (Math|Vector|Lerp(Vector) (Variables|/Script/Engine.SceneComponent|GetRelativeLocation (Variables|Default|GetSlider)) (.Position (Utilities|Struct|BreakSplinePoint (Spline|GetSplinePointAt (Variables|Default|GetSpline) (Variables|Default|GetPoint%20Index) "Local"))) _alpha) false false)))
          (else
            (Timeline|SliderAnim PlayFromStart)))))))

(event EventBeginPlay
  (Transformation|SetRelativeLocation (Variables|Default|GetSlider) (.Position (Utilities|Struct|BreakSplinePoint (Spline|GetSplinePointAt (Variables|Default|GetSpline) 0 "Local"))) false false)
  (bind _returnvalue (Actor|GetActorOfClass "/Game/Game/Blueprints/GPE/BP_ConsoleSlider.BP_ConsoleSlider_C"))
  (Variables|Default|SetConsole _returnvalue)
  (Components|Timeline|SetPlayRate (Variables|Default|GetSliderAnim) 5.0))

(event Collision|EventActorBeginOverlap
  (params (OtherActor :type Actor%20Object%20Reference)))

(event EventTick
  (params (DeltaSeconds :type Float%20%28single-precision%29)))

(fn ConstructionScript)

(fn CheckPos
  (return (Variables|Default|GetPoint%20Index)))