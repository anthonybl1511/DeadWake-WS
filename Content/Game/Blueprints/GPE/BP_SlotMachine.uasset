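; BP_SlotMachine is an interactable lever that stays jammed until powered, then reports its slot state to the lab door.
; Activated enables electricity and reveals a point light.
; When powered, interaction toggles the lever through a forward/reverse timeline with sounds, passing SlotID and Down to the BP_LabDoor found on BeginPlay when movement finishes.
; Without power, two short timelines nudge the lever and back, with sparks and a stuck sound.
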(event OnInteractionBegin(Manager_InteractionTarget)
  (params (InteractorPawn :type Pawn%20Object%20Reference))
  (bind _initial_rotation (Variables|Default|GetInitial%20rotation))
  (bind _initial_rotation_2 (Variables|Default|GetInitial%20rotation))
  (bind _initial_rotation_3 (Variables|Default|GetInitial%20rotation))
  (bind (_roll _pitch _yaw) (Math|Rotator|BreakRotator _initial_rotation))
  (bind (_roll_2 _pitch_2 _yaw_2) (Math|Rotator|BreakRotator _initial_rotation_2))
  (bind (_roll_3 _pitch_3 _yaw_3) (Math|Rotator|BreakRotator _initial_rotation_3))
  (if (Variables|Default|GethasEletricity?)
    (if (not (Variables|Default|GetDown?))
      (Audio|PlaySoundatLocation "/Game/Game/SFX/SFX_Lever.SFX_Lever" (Transformation|GetWorldLocation (Variables|Default|GetSlotMachine)) "0, 0, 0" 1.0 1.0 0.0 "/Game/Game/Blueprints/GPE/SA_GeneralSettings.SA_GeneralSettings" 0 0 0)
      (Variables|Default|SetDown? true)
      (bind _alpha (Timeline|LeverAnim PlayFromStart)
        (:Update
          (Transformation|SetRelativeRotation (Variables|Default|GetManivelle) (Math|Rotator|Lerp(Rotator) _initial_rotation (Math|Rotator|MakeRotator (+ _roll -5e+01) _pitch _yaw) _alpha true) false false))
        (:Finished
          (Default|GetSlotState (Variables|Default|GetDoor) (Variables|Default|GetSlotID) (Variables|Default|GetDown?))))
      (else
        (Audio|PlaySoundatLocation "/Game/Game/SFX/SFX_LeverUp__online-audio-converter_com_.SFX_LeverUp__online-audio-converter_com_" (Transformation|GetWorldLocation (Variables|Default|GetSlotMachine)) "0, 0, 0" 1.0 1.0 0.0 "/Game/Game/Blueprints/GPE/SA_GeneralSettings.SA_GeneralSettings" 0 0 0)
        (Variables|Default|SetDown? false)
        (Timeline|LeverAnim ReverseFromEnd)))
    (else
      ;[1 0 0.01747] Incorrect/Not working sound
      (Audio|PlaySoundatLocation "/Game/Game/SFX/SFX_StuckLever.SFX_StuckLever" (Transformation|GetWorldLocation (Variables|Default|GetSlotMachine)) "0, 0, 0" 1.0 1.0 0.5 0 0 0 0)
      (Audio|PlaySoundatLocation 0 (Transformation|GetWorldLocation (Variables|Default|GetSlotMachine)) "0, 0, 0" 1.0 1.0 0.0 "/Game/Game/Blueprints/GPE/SA_GeneralSettings.SA_GeneralSettings" 0 0 0)
      (Components|Activation|Activate (Variables|Default|GetP_Sparks_C) true)
      (bind _alpha_2 (Timeline|BlockAnim1 PlayFromStart)
        (:Update
          (Transformation|SetRelativeRotation (Variables|Default|GetManivelle) (Math|Rotator|Lerp(Rotator) _initial_rotation_2 (Math|Rotator|MakeRotator (+ _roll_2 -1e+01) _pitch_2 _yaw_2) _alpha_2 true) false false))
        (:Finished
          (bind _alpha_3 (Timeline|BlockAnim2 ReverseFromEnd)
            (:Update
              (Transformation|SetRelativeRotation (Variables|Default|GetManivelle) (Math|Rotator|Lerp(Rotator) _initial_rotation_3 (Math|Rotator|MakeRotator (+ _roll_3 -1e+01) _pitch_3 _yaw_3) _alpha_3 true) false false))))))))

(event Custom|Activated
  (Variables|Default|SethasEletricity? true)
  (Development|SetHiddeninGame (Variables|Default|GetPointLight) false false))

(event EventBeginPlay
  (Variables|Default|SetInitial%20rotation (Variables|/Script/Engine.SceneComponent|GetRelativeRotation (Variables|Default|GetManivelle)))
  (Components|Timeline|SetPlayRate (Variables|Default|GetLeverAnim) 2.0)
  (Variables|Default|SethasEletricity? false)
  (Components|Timeline|SetPlayRate (Variables|Default|GetBlockAnim1) 3.0)
  (Components|Timeline|SetPlayRate (Variables|Default|GetBlockAnim2) 3.0)
  (bind _returnvalue (Actor|GetActorOfClass "/Game/Game/Blueprints/GPE/BP_LabDoor.BP_LabDoor_C"))
  (Variables|Default|SetDoor _returnvalue)
  (Development|SetHiddeninGame (Variables|Default|GetPointLight) true false))

(event Collision|EventActorBeginOverlap
  (params (OtherActor :type Actor%20Object%20Reference)))

(event EventTick
  (params (DeltaSeconds :type Float%20%28single-precision%29)))

(fn ConstructionScript)