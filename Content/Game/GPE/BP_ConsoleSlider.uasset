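; BP_ConsoleSlider is a console puzzle that checks slider positions against a combination.
; BeginPlay fills an array of three indicators.
; CheckPos compares each slider's PointIndex to Combination, turning matches green and adjusting a CorrectSlider counter that persists between checks, with only a debug print at three.
; Mismatches apply red to the first indicator, using the slider index as material slot, rather than to the matching indicator.
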(event Custom|CheckPos
  (for (_array_element _array_index) (Variables|Default|GetSliders)
    (if (== (Variables|/Game/Game/GPE/BP_Slider.BP_Slider_C|GetPoint%20Index _array_element) (Utilities|Array|Get(acopy) (Variables|Default|GetCombination) _array_index))
      (Rendering|Material|SetMaterial (Utilities|Array|Get(acopy) (Variables|Default|GetIndicators) _array_index) 0 "/Game/Game/GPE/PlaceholderMaterials/MI_Green.MI_Green")
      (Development|PrintString "adding one")
      (bind _result (Math|Integer|IncrementInt (Variables|Default|GetCorrectSlider))
        (:%20%20
          (if (== _result 3)
            (Development|PrintString "Good"))))
      (else
        (Rendering|Material|SetMaterial (Utilities|Array|Get(acopy) (Variables|Default|GetIndicators)) _array_index "/Game/Game/GPE/PlaceholderMaterials/MI_Red.MI_Red")
        (bind _result_2 (Math|Integer|DecrementInt (Variables|Default|GetCorrectSlider))
          (:%20%20
            (if (< _result_2 0)
              (Variables|Default|SetCorrectSlider 0)))))))
  (Development|PrintString (Utilities|String|ToString(Integer) (Variables|Default|GetCorrectSlider))))

(event Collision|EventActorBeginOverlap
  (params (OtherActor :type Actor%20Object%20Reference)))

(event EventTick
  (params (DeltaSeconds :type Float%20%28single-precision%29)))

(event EventBeginPlay
  (bind _indicators (Variables|Default|GetIndicators))
  (Utilities|Array|SetArrayElem _indicators 0 (Variables|Default|GetIndicator1) true)
  (Utilities|Array|SetArrayElem _indicators 1 (Variables|Default|GetIndicator2) true)
  (Utilities|Array|SetArrayElem _indicators 2 (Variables|Default|GetIndicator3) true)
  (Development|PrintString (Utilities|GetDisplayName (Utilities|Array|Get(acopy) _indicators))))

(fn ConstructionScript)