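; BP_Slider is an interactable puzzle-style element whose slider steps along spline points each time it is used.
; Each interaction increments PointIndex, notifies the Console through its CheckPos, and plays a timeline that lerps the slider from its current location toward that point.
; The index resets to zero after the move to the fifth point finishes.
; Its own CheckPos function exposes the current index.
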(event OnInteractionBegin(Manager_InteractionTarget)
  (params (InteractorPawn :type Pawn%20Object%20Reference))
  (Math|Integer|IncrementInt (Variables|Default|GetPoint%20Index)
    (:%20%20
      (Default|CheckPos (Variables|Default|GetConsole))
      (bind _alpha (Timeline|SliderAnim PlayFromStart)
        (:Update
          (Transformation|SetRelativeLocation (Variables|Default|GetSlider) (Math|Vector|Lerp(Vector) (Variables|/Script/Engine.SceneComponent|GetRelativeLocation (Variables|Default|GetSlider)) (.Position (Utilities|Struct|BreakSplinePoint (Spline|GetSplinePointAt (Variables|Default|GetSpline) (Variables|Default|GetPoint%20Index) "Local"))) _alpha) false false))
        (:Finished
          (if (>= (Variables|Default|GetPoint%20Index) 5)
            (Variables|Default|SetPoint%20Index 0)))))))

(event EventBeginPlay
  (Transformation|SetRelativeLocation (Variables|Default|GetSlider) (.Position (Utilities|Struct|BreakSplinePoint (Spline|GetSplinePointAt (Variables|Default|GetSpline) 0 "Local"))) false false))

(event Collision|EventActorBeginOverlap
  (params (OtherActor :type Actor%20Object%20Reference)))

(event EventTick
  (params (DeltaSeconds :type Float%20%28single-precision%29)))

(fn ConstructionScript)

(fn CheckPos
  (return (Variables|Default|GetPoint%20Index)))